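; BP_Light is a trigger light actor that switches on when its Box is first overlapped and counts toward the lights the player has passed.
; A DoOnce on the overlap sets the Lighting flag, increments PassedLights on BP_myGamemode and prints the new total, without filtering the overlapping actor.
; Tick applies the Lighting flag to the PointLight's visibility every frame.
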(event `self.ReceiveTick`
  (params (DeltaSeconds :type "Float (single-precision)"))
  (`SceneComponent.SetVisibility` (`self.PointLight`) (`self.Lighting`) false))

(event `self.Box.OnComponentBeginOverlap`
  (params (OverlappedComponent :type "PrimitiveComponent Object Reference") (OtherActor :type "Actor Object Reference") (OtherComp :type "PrimitiveComponent Object Reference") (OtherBodyIndex :type Integer) (bFromSweep :type Boolean) (SweepResult :type "HitResult Structure (by ref)"))
  (`/Engine/EditorBlueprintResources/StandardMacros.DoOnce` false
    (:`Completed`
      (set `self.Lighting` true)
      (bind _asbp_my_gamemode (cast `/Game/blueprints/BP_myGamemode` (`GameplayStatics.GetGameMode`)))
      (bind _output_get (set `/Game/blueprints/BP_myGamemode.passedLights` (+ (`/Game/blueprints/BP_myGamemode.passedLights` _asbp_my_gamemode) 1) _asbp_my_gamemode))
      (`KismetSystemLibrary.PrintString` (`KismetStringLibrary.Conv_IntToString` _output_get)))))

(fn `UserConstructionScript`)